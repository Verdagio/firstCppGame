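; Weapon Blueprint actor that provides automatic fire by spawning Bullet actors at an Arrow component's transform.
; PullTrig passes through a DoOnce, fires immediately, then starts a looping timer on Shoot with an interval derived from Time divided by Rps.
; ReleaseTrig clears that timer to stop firing but does not reset the DoOnce, so later pulls do not fire again.
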(event Custom|PullTrig
  ;[1 1 1] Event handler for pulling the trigger
  (Utilities|FlowControl|DoOnce false
    (:Completed
      (CallFunction|Shoot)
      (Utilities|Time|SetTimerbyFunctionName 0 "Shoot" (/ (Variables|Default|GetTime) (Variables|Default|GetRps)) true))))

(event Custom|ReleaseTrig
  ;[1 1 1] Stops firing once trigger released
  (Utilities|Time|ClearTimerbyFunctionName 0 "Shoot"))

(event Custom|Shoot
  ;[1 1 1] Shooting mechanic
  (Game|SpawnActorfromClass "/Game/BluePrints/bullet.bullet_C" (Transformation|GetWorldTransform (Variables|Default|GetArrow)) "Undefined" 0 0))

(event EventBeginPlay)

(event Collision|EventActorBeginOverlap
  (params (OtherActor :type Actor%20Object%20Reference)))

(event EventTick
  (params (DeltaSeconds :type Float%20%28single-precision%29)))

(fn ConstructionScript)