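; MapGenerator is an actor Blueprint that lays out a flat rectangular grid of floor tiles.
; Its construction script adds MaX by MaxY instances to the Floor instanced mesh component, spaced by TileSize at local zero height.
; A single loop derives each tile's X and Y cell from the index using integer division and modulo.
; The event graph holds only disabled placeholder events, so no runtime logic exists.
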(event EventBeginPlay)

(event Collision|EventActorBeginOverlap
  (params (OtherActor :type Actor%20Object%20Reference)))

(event EventTick
  (params (DeltaSeconds :type Float%20%28single-precision%29)))

(fn ConstructionScript
  (bind _maxy (Variables|Default|GetMaxY))
  (bind _tilesize (Variables|Default|GetTileSize))
  (for _index (range 0 (- (* (Variables|Default|GetMa\X) (Variables|Default|GetMaxY)) 1))
    (Components|InstancedStaticMesh|AddInstance (Variables|Default|Getfloor) (Math|Conversions|ToTransform(Vector) (Math|Vector|MakeVector (Math|Conversions|ToFloat(Integer) (* (/ _index _maxy) _tilesize)) (Math|Conversions|ToFloat(Integer) (* (Math|Integer|%(Integer) _index _maxy) _tilesize)) 0.0)))))