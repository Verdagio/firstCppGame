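; EnemySpawn is a spawner actor that periodically spawns AI Enemy pawns inside its Box volume.
; BeginPlay looks up the first EnemySpawn in the level and sets a looping SpawnEnemy timer on it, so additional spawners target that same instance.
; The interval is Time divided by EnemiesPerSec.
; Each SpawnEnemy call spawns at a random point in the box while the world's Enemy count is below MaxEnemies.
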(event Custom|SpawnEnemy
  (bind _box (Variables|Default|GetBox))
  ;[1 1 1] This will get all instances of the Enemy class and restrict the number that will allowed to be spawned
  (bind _outactors (Actor|GetAllActorsOfClass "/Game/BluePrints/Enemy.Enemy_C"))
  (if (< (Utilities|Array|Length _outactors) (Variables|Default|GetMaxEnemies))
    (AI|SpawnAIFromClass "/Game/BluePrints/Enemy.Enemy_C" 0 (Math|Random|RandomPointinBoundingBox (Transformation|GetWorldLocation _box) (Components|Box|GetScaledBoxExtent _box)) "0, 0, 0" false)))

(event EventBeginPlay
  (bind _outactors (Actor|GetAllActorsOfClass "EnemySpawn_C"))
  (bind _output_get (Variables|EnemySpawn_C|SetNewVar_0 (Utilities|Array|Get(acopy) _outactors) (Utilities|Array|Get(acopy) _outactors)))
  (Utilities|Time|SetTimerbyFunctionName _output_get "SpawnEnemy" (/ (Variables|Default|Gettime) (Variables|Default|GetEnemiesPerSec)) true))

(event Collision|EventActorBeginOverlap
  (params (OtherActor :type Actor%20Object%20Reference)))

(event EventTick
  (params (DeltaSeconds :type Float%20%28single-precision%29)))

(fn ConstructionScript)