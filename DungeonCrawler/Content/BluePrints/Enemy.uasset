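; Enemy actor that deals repeated damage to the Player while overlapping it and can take damage itself.
; Overlapping a Player starts a looping one-second timer that calls the Player's AffectHealth, and ending the overlap clears it.
; Its own AffectHealth passes the delta to CheckHealth, then destroys the actor on the branch where IsAlive is true.
; The construction script tints the mesh with EnemyColour through a dynamic material instance.
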(event Custom|DamagePlayer
  ;[1 1 1] Damage the player
  (Default|AffectHealth (Variables|Default|Getplayer) (Variables|Default|Getdamage)))

(event EventBeginPlay)

(event Collision|EventActorBeginOverlap
  (params (OtherActor :type Actor%20Object%20Reference))
  ;[1 1 1] Damage the player
  (bind _asplayer (Utilities|Casting|CastToPlayer OtherActor))
  (Variables|Default|Setplayer _asplayer)
  (Utilities|Time|SetTimerbyFunctionName 0 "DamagePlayer" 1.0 true))

(event EventTick
  (params (DeltaSeconds :type Float%20%28single-precision%29)))

(event Collision|EventActorEndOverlap
  (params (OtherActor :type Actor%20Object%20Reference))
  ;[1 1 1] Damage the player
  (if (== OtherActor (Variables|Default|Getplayer))
    (Utilities|Time|ClearTimerbyFunctionName 0 "DamagePlayer")))

(event EventAffectHealth
  (params (Delta :type Float%20%28single-precision%29))
  ;[1 1 1] Damage this character
  (Class|BaseCharacter|CheckHealth Delta)
  (if (Variables|Default|GetisAlive)
    (Actor|DestroyActor)))

(fn ConstructionScript
  (bind _returnvalue (Rendering|Material|CreateDynamicMaterialInstance (Variables|Character|GetMesh) 0 0 :!class /Script/Engine.PrimitiveComponent))
  (bind _output_get (Variables|Default|SetDynamic%20Material _returnvalue))
  (Rendering|Material|SetVectorParameterValue _output_get "BodyColor" (Variables|Default|GetEnemyColour) :!class /Script/Engine.MaterialInstanceDynamic))