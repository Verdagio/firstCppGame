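; Floor Blueprint that procedurally lays out a tiled floor with walls segmenting it into a grid, as groundwork for rooms.
; Its construction script uses nested loops to add Floor, WallX and WallY mesh instances spaced by TileSize.
; WallX loops use only LastX and WallY only LastY with negated Y offsets, so each forms a square grid.
; An earlier perimeter-wall pass is left disconnected, and the event graph is empty.
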(event EventBeginPlay)

(event Collision|EventActorBeginOverlap
  (params (OtherActor :type Actor%20Object%20Reference)))

(event EventTick
  (params (DeltaSeconds :type Float%20%28single-precision%29)))

(fn ConstructionScript
  (bind _lastx (Variables|Default|GetLastX))
  (bind _lasty (Variables|Default|GetLastY))
  (bind _returnvalue (+ _lastx 1))
  (bind _returnvalue_2 (+ _lasty 1))
  (Utilities|FlowControl|Sequence
    (:then_0
      ;[1 1 1] 1 -To create the floor - loop from 0 - max X & 0 - max Y, multiply the index of each by the tile size to get the x & y locations which will be passed into our vector, then to the instance transfrom for each floor mesh instance
      (for _index (range 0 (Variables|Default|GetLastX))
        (for _index_2 (range 0 (Variables|Default|GetLastY))
          (Components|InstancedStaticMesh|AddInstance (Variables|Default|GetFloor) (Math|Transform|MakeTransform (Math|Vector|MakeVector (Math|Conversions|ToFloat(Integer) (* _index (Variables|Default|GetTileSize))) (Math|Conversions|ToFloat(Integer) (* _index_2 (Variables|Default|GetTileSize))) 0.0))))))
    (:then_1
      ;[1 1 1] Add walls that will surround and segment the space into a grid, next step knock some walls... or place rooms within the space replacing walls to make rooms...then create doorways..
      (for _index_3 (range 0 _returnvalue_2)
        (for _index_4 (range 0 _returnvalue_2)
          (Components|InstancedStaticMesh|AddInstance (Variables|Default|GetWallY) (Math|Conversions|ToTransform(Vector) (Math|Vector|MakeVector (Math|Conversions|ToFloat(Integer) (* _index_4 (Variables|Default|GetTileSize))) (Math|Conversions|ToFloat(Integer) (* _index_3 (* (Variables|Default|GetTileSize) -1))) 0.0))))))
    (:then_2
      (for _index_5 (range 0 _returnvalue)
        (for _index_6 (range 0 _returnvalue)
          (Components|InstancedStaticMesh|AddInstance (Variables|Default|GetWallX) (Math|Conversions|ToTransform(Vector) (Math|Vector|MakeVector (Math|Conversions|ToFloat(Integer) (* _index_6 (Variables|Default|GetTileSize))) (Math|Conversions|ToFloat(Integer) (* _index_5 (Variables|Default|GetTileSize))) 0.0))))))
    (:then_3)))