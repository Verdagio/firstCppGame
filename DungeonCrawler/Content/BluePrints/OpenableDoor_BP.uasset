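; OpenableDoor_BP is a door actor that swings open and closed when DoorControl fires its OnOpen and OnClose events.
; The OpenTime timeline plays forward to open and reverses to close, driving a yaw angle combined with the rotation saved at BeginPlay.
; An event track on the same timeline plays the DoorLock sound at the actor's location.
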(event OnClose(DoorControl)
  (bind _angle (Timeline|openTime Reverse)
    (:Update
      (Transformation|SetActorRotation (Math|Rotator|CombineRotators (Math|Rotator|MakeRotator 0.0 0.0 _angle) (Variables|Default|GetInit%20Rotation))))
    (:sound%20time
      (Audio|PlaySoundatLocation "/Game/Audio/doorLock.doorLock" (Transformation|GetActorLocation)))))

(event OnOpen(DoorControl)
  (bind _angle (Timeline|openTime Play)
    (:Update
      (Transformation|SetActorRotation (Math|Rotator|CombineRotators (Math|Rotator|MakeRotator 0.0 0.0 _angle) (Variables|Default|GetInit%20Rotation))))
    (:sound%20time
      (Audio|PlaySoundatLocation "/Game/Audio/doorLock.doorLock" (Transformation|GetActorLocation)))))

(event EventBeginPlay
  (Variables|Default|SetInit%20Rotation (Transformation|GetActorRotation)))

(fn ConstructionScript)